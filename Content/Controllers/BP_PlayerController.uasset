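; Player controller that moves the controlled pawn, turns the camera and places anchors at the cursor.
; Forward and Right axes drive movement along the pawn's own forward and right vectors.
; TurnCamera yaw input passes through a gate that LockCameraRotation opens on press and closes on release.
; CreateAnchor spawns an actor at the cursor's hit location on a single object type, owned by the hit actor.
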(event Input|ActionEvents|InputActionLockCameraRotation
  (params (Key :type Key%20Structure))
  (:Pressed
    (Utilities|FlowControl|Gate true) ; enters at Open
  )
  (:Released
    (Utilities|FlowControl|Gate true) ; enters at Close
  ))

(event Input|ActionEvents|InputActionCreateAnchor
  (params (Key :type Key%20Structure))
  (bind _array (Utilities|Array|MakeArray "ObjectTypeQuery7"))
  (bind _hitresult (Class|PlayerController|GetHitResultUnderCursorforObjects _array false))
  (bind (_bblockinghit _binitialoverlap _time _distance _location _impactpoint _normal _impactnormal _physmat _hitactor) (Collision|BreakHitResult _hitresult))
  (:Pressed
    (Game|SpawnActorfromClass "/Game/Actors/Anchor.Anchor_C" (Math|Transform|MakeTransform _location) "AlwaysSpawn" _hitactor 0)))

(event Input|AxisEvents|InputAxisForward
  (params (AxisValue :type Float%20%28single-precision%29))
  (bind _returnvalue (Pawn|GetControlledPawn))
  (Pawn|Input|AddMovementInput _returnvalue (Transformation|GetActorForwardVector _returnvalue) AxisValue false))

(event Input|AxisEvents|InputAxisRight
  (params (AxisValue :type Float%20%28single-precision%29))
  (bind _returnvalue (Pawn|GetControlledPawn))
  (Pawn|Input|AddMovementInput _returnvalue (Transformation|GetActorRightVector _returnvalue) AxisValue false))

(event Input|AxisEvents|InputAxisTurnCamera
  (params (AxisValue :type Float%20%28single-precision%29))
  (Utilities|FlowControl|Gate true
    (:Exit
      (Class|PlayerController|AddYawInput AxisValue))))

(fn ConstructionScript)