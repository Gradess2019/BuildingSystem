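; Player controller that maps movement and camera turn input to the controlled pawn.
; Forward and Right axes add movement input along the pawn's forward and right vectors.
; TurnCamera adds yaw input only through a gate that the LockCameraRotation action opens while held and closes on release, so the camera turns only during the hold.
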(event Input|ActionEvents|InputActionLockCameraRotation
  (params (Key :type Key%20Structure))
  (:Pressed
    (Utilities|FlowControl|Gate true) ; enters at Open
  )
  (:Released
    (Utilities|FlowControl|Gate true) ; enters at Close
  ))

(event Input|AxisEvents|InputAxisForward
  (params (AxisValue :type Float%20%28single-precision%29))
  (bind _returnvalue (Pawn|GetControlledPawn))
  (Pawn|Input|AddMovementInput _returnvalue (Transformation|GetActorForwardVector _returnvalue) AxisValue false))

(event Input|AxisEvents|InputAxisRight
  (params (AxisValue :type Float%20%28single-precision%29))
  (bind _returnvalue (Pawn|GetControlledPawn))
  (Pawn|Input|AddMovementInput _returnvalue (Transformation|GetActorRightVector _returnvalue) AxisValue false))

(event Input|AxisEvents|InputAxisTurnCamera
  (params (AxisValue :type Float%20%28single-precision%29))
  (Utilities|FlowControl|Gate true
    (:Exit
      (Class|PlayerController|AddYawInput AxisValue))))

(fn ConstructionScript)